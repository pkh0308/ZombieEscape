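; BP_TestZombie is a test zombie enemy that damages the player on contact and can be killed by bullets.
; An attack collision overlap applies its attack power to a PlayerCharacter through that character's OnDamaged.
; A capsule overlap with a Bullet deals fixed damage to the zombie through its own OnDamaged.
; Health starts at max, stays clamped, and the actor destroys itself through OnDie when it reaches zero.
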(event OnComponentBeginOverlap(AttackCollision)
  (params (OverlappedComponent :type Primitive%20Component%20Object%20Reference) (OtherActor :type Actor%20Object%20Reference) (OtherComp :type Primitive%20Component%20Object%20Reference) (OtherBodyIndex :type Integer) (bFromSweep :type Boolean) (SweepResult :type Hit%20Result%20Structure%20%28by%20ref%29))
  (bind _asplayer_character (Utilities|Casting|CastToPlayerCharacter OtherActor))
  (Class|PlayerCharacter|OnDamaged _asplayer_character (Variables|Default|GetAttackPower)))

(event OnComponentBeginOverlap(CapsuleComponent)
  (params (OverlappedComponent :type Primitive%20Component%20Object%20Reference) (OtherActor :type Actor%20Object%20Reference) (OtherComp :type Primitive%20Component%20Object%20Reference) (OtherBodyIndex :type Integer) (bFromSweep :type Boolean) (SweepResult :type Hit%20Result%20Structure%20%28by%20ref%29))
  (Utilities|Casting|CastToBullet OtherActor)
  (CallFunction|OnDamaged 10))

(event EventBeginPlay
  ;[1 1 1] Initilalize
  (Variables|Default|SetCurHp (Variables|Default|GetMaxHp)))

(event Collision|EventActorBeginOverlap
  (params (OtherActor :type Actor%20Object%20Reference)))

(event EventTick
  (params (DeltaSeconds :type Float%20%28single-precision%29)))

(fn ConstructionScript)

(fn OnDamaged
  (params (InDamage :type Integer))
  (bind _output_get (Variables|Default|SetCurHp (Math|Integer|Clamp(Integer) (- (Variables|Default|GetCurHp) InDamage) 0 (Variables|Default|GetMaxHp))))
  (if (== _output_get 0)
    (CallFunction|OnDie)))

(fn OnDie
  (Actor|DestroyActor))